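; Horde spawner actor that spawns charger enemies off-screen, each given either a random or a specified paint colour.
; triggerHorde stores the colour choice and starts a timer on spawnNewEnemy, which re-arms itself after each spawn until disableHorde clears IsSpawning.
; IsInView projects the spawner's location against viewport bounds to block on-screen spawns.
; An on-screen check skips re-arming, so the chain stops while IsSpawning stays true.
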(event `triggerHorde`
  (params (isRandom :type Boolean) (isColour :type "/Game/paint/enum_Paint Enum"))
  (if (not (`self.isSpawning`))
    (set `self.randomColour` isRandom)
    (set `self.spawnColour` isColour)
    (set `self.isSpawning` true)
    (`KismetSystemLibrary.K2_SetTimer` self "spawnNewEnemy" 5.0)))

(event `disableHorde`
  (set `self.isSpawning` false))

(fn `isInView`
  (returns (truth :type Boolean))
  (bind (_returnvalue_x _returnvalue_y) (`KismetMathLibrary.BreakVector2D` (`WidgetLayoutLibrary.GetViewportSize`)))
  (bind _screenposition (`GameplayStatics.ProjectWorldToScreen` (`GameplayStatics.GetPlayerController` 0) (`SceneComponent.K2_GetComponentLocation` (`self.DefaultSceneRoot`))))
  (bind _returnvalue (and (< 0.0 (`KismetMathLibrary.BreakVector2D` _screenposition)) (< 0.0 (`.Y` (`KismetMathLibrary.BreakVector2D` _screenposition))) (< (`KismetMathLibrary.BreakVector2D` _screenposition) _returnvalue_x) (< (`.Y` (`KismetMathLibrary.BreakVector2D` _screenposition)) _returnvalue_y)))
  ;[1 1 1] Detects where the object is relative to player camera
  (if _returnvalue
    _
    (else
      _))
  (return _returnvalue))

(fn `spawnNewEnemy`
  (bind _truth (`self.isInView`))
  (if _truth
    _
    (elif (`self.isSpawning`)
      (bind _returnvalue (`|SpawnActorFromClass` "/Game/enemy/bp_enemyCharger.bp_enemyCharger_C" (`SceneComponent.GetRelativeTransform` (`self.DefaultSceneRoot`)) "AlwaysSpawn" "OverrideRootScale"))
      ;[1 1 1] Spawns with specific colour if allowed, else chooses random
      (if (`self.randomColour`)
        (`/Game/enemy/bp_enemyTest.setEnemyColour` _returnvalue (cast `/Game/paint/enum_Paint` (`KismetMathLibrary.Conv_IntToByte` (`KismetMathLibrary.RandomIntegerInRange` 0 3))))
        (else
          (`/Game/enemy/bp_enemyTest.setEnemyColour` _returnvalue (`self.spawnColour`))))
      (`KismetSystemLibrary.K2_SetTimer` self "spawnNewEnemy" 5.0))))

(fn `UserConstructionScript`)