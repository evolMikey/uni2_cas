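; Paint-coloured enemy for a twin-stick game that spawns its own AI controller and chases the player's pawn every tick via AI MoveTo.
; setEnemyColour stores one of four paint types and pushes its colour into the UFO mesh's pColour material parameter.
; Lethal damage plays a pop, leaves a matching paint decal and splat emitter, awards points, then destroys the actor.
; HitPlayer does the same without awarding points.
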(event `self.ReceiveBeginPlay`
  (`self.SpawnDefaultController`))

(event `setEnemyColour`
  (params (newPaint :type "/Game/paint/enum_Paint Enum"))
  ;[1 1 1] Switches the enemy colour, mostly used during spawning
  (`self.setDataColour` newPaint
    (:`output`
      (`self.setMatColour`))))

(event `enemy_takeDamage`
  (params (damageVal :type "Float (double-precision)"))
  ;[1 1 1] Applies damage to enemy
  (bind _output_get (set `self.enemyHealth` (- (`self.enemyHealth`) damageVal)))
  (if (<= _output_get 0.0)
    (`GameplayStatics.PlaySoundAtLocation` "/Game/Sounds/Enemy_death_Pop.Enemy_death_Pop" (`self.K2_GetActorLocation` self))
    (`self.deathDecal`
      (:`output`
        (`self.givePoints`
          (:`output`
            (`self.K2_DestroyActor`)))))))

(event `self.ReceiveTick`
  (params (DeltaSeconds :type "Float (single-precision)"))
  (`|AIMoveTo` self (`self.K2_GetActorLocation` (`Controller.K2_GetPawn` (`GameplayStatics.GetPlayerController` 0))) null 10.0))

(event `HitPlayer`
  (params (damageVal :type "Float (double-precision)"))
  ;[1 1 1] Applies damage to enemy
  (`GameplayStatics.PlaySoundAtLocation` "/Game/Sounds/Enemy_death_Pop.Enemy_death_Pop" (`self.K2_GetActorLocation`))
  (`self.deathDecal`
    (:`output`
      (`self.K2_DestroyActor`))))

(fn `UserConstructionScript`)