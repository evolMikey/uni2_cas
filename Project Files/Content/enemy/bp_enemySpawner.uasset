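; Enemy spawner that, once triggered, spawns a set number of paint-coloured test enemies at its location while off screen.
; triggerSpawning stores the count and a fixed or random colour, then starts a repeating timer on SpawnNewEnemy until the count runs out or disableSpawning clears the flag.
; IsInView projects the spawner to screen space against viewport bounds, delaying spawns while visible and printing a debug string on each check.
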(event `triggerSpawning`
  (params (isRandom :type Boolean) (isColour :type "/Game/paint/enum_Paint Enum") (numSpawn :type Integer))
  ;[1 1 1] Enables this spawner and gives it a few variables to work with
  (if (not (`self.isSpawning`))
    ;;[1 1 1] Is colour chosen randomly? Else set colour
    (bind _output_get (set `self.randomColour` isRandom))
    (if (not _output_get)
      (set `self.spawnColour` isColour))
    ;;[1 1 1] Number to spawn
    (set `self.spawnNumber` numSpawn)
    ;;[1 1 1] Enables spawning
    (set `self.isSpawning` true)
    (`KismetSystemLibrary.K2_SetTimer` self "spawnNewEnemy" 5.0)))

(event `disableSpawning`
  (set `self.isSpawning` false))

(fn `IsInView`
  (returns (truth :type Boolean))
  (bind (_returnvalue_x _returnvalue_y) (`KismetMathLibrary.BreakVector2D` (`WidgetLayoutLibrary.GetViewportSize`)))
  (bind _screenposition (`GameplayStatics.ProjectWorldToScreen` (`GameplayStatics.GetPlayerController` 0) (`SceneComponent.K2_GetComponentLocation` (`self.DefaultSceneRoot`))))
  (bind _returnvalue (and (< 0.0 (`KismetMathLibrary.BreakVector2D` _screenposition)) (< 0.0 (`.Y` (`KismetMathLibrary.BreakVector2D` _screenposition))) (< (`KismetMathLibrary.BreakVector2D` _screenposition) _returnvalue_x) (< (`.Y` (`KismetMathLibrary.BreakVector2D` _screenposition)) _returnvalue_y)))
  ;[1 1 1] Detects where the object is relative to player camera
  (if _returnvalue
    (`KismetSystemLibrary.PrintString` "TRUTH")
    (else
      (`KismetSystemLibrary.PrintString` "FALSE")))
  (return _returnvalue))

(fn `spawnNewEnemy`
  (bind _spawnnumber (`self.spawnNumber`))
  ;[1 1 1] Checks that conditions are met to start spawning, removes one from spawn counter
  (bind _truth (`self.IsInView`))
  (if _truth
    ;[1 1 1] Calls this function again, will only cease once counter reaches 0
    (`KismetSystemLibrary.K2_SetTimer` self "spawnNewEnemy" 5.0)
    (elif (`self.isSpawning`)
      (if (> _spawnnumber 0)
        (`/Engine/EditorBlueprintResources/StandardMacros.DecrementInt` _spawnnumber
          (:`  `
            ;[1 1 1] Spawns new enemy character on spawner location
            (bind _returnvalue (`|SpawnActorFromClass` "/Game/enemy/bp_enemyTest.bp_enemyTest_C" (`SceneComponent.GetRelativeTransform` (`self.DefaultSceneRoot`)) "AlwaysSpawn" "OverrideRootScale"))
            ;[1 1 1] Spawns with specific colour if allowed, else chooses random
            (if (`self.randomColour`)
              (`/Game/enemy/bp_enemyTest.setEnemyColour` _returnvalue (cast `/Game/paint/enum_Paint` (`KismetMathLibrary.Conv_IntToByte` (`KismetMathLibrary.RandomIntegerInRange` 0 3))))
              (else
                (`/Game/enemy/bp_enemyTest.setEnemyColour` _returnvalue (`self.spawnColour`))))
            ;[1 1 1] Calls this function again, will only cease once counter reaches 0
            (`KismetSystemLibrary.K2_SetTimer` self "spawnNewEnemy" 5.0)))))))

(fn `UserConstructionScript`)